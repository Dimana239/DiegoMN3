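; BP_Checkpoint is a checkpoint actor with a sphere trigger that records the player's last saved location.
; When a BP_ThirdPersonCharacter overlaps the sphere, it writes the sphere's world location to that character's LastSavedLocation and activates the CheckpointSystem component with reset.
; It then casts the game instance to GL_SaveLoad and calls LoadGame twice in succession, with no save call in this graph.
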(event OnComponentBeginOverlap(Sphere)
  (params (OverlappedComponent :type Primitive%20Component%20Object%20Reference) (OtherActor :type Actor%20Object%20Reference) (OtherComp :type Primitive%20Component%20Object%20Reference) (OtherBodyIndex :type Integer) (bFromSweep :type Boolean) (SweepResult :type Hit%20Result%20Structure%20%28by%20ref%29))
  (bind _asbp_third_person_character (Utilities|Casting|CastToBP_ThirdPersonCharacter OtherActor))
  (Variables|/Game/ThirdPerson/Blueprints/BP_ThirdPersonCharacter.BP_ThirdPersonCharacter_C|SetLastSavedLocation _asbp_third_person_character (Transformation|GetWorldLocation (Variables|Default|GetSphere)))
  (Components|Activation|Activate (Variables|Default|GetCheckpointSystem) true)
  (bind _asgl_save_load (Utilities|Casting|CastToGL_SaveLoad (Game|GetGameInstance)))
  (Default|LoadGame _asgl_save_load)
  (bind _asgl_save_load_2 (Utilities|Casting|CastToGL_SaveLoad (Game|GetGameInstance)))
  (Default|LoadGame _asgl_save_load_2))

(event EventBeginPlay)

(event Collision|EventActorBeginOverlap
  (params (OtherActor :type Actor%20Object%20Reference)))

(event EventTick
  (params (DeltaSeconds :type Float%20%28single-precision%29)))

(fn ConstructionScript)