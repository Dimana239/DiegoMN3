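; Game mode that manages per-level save data, using the current level name as the save slot.
; On BeginPlay it loads or creates an SG_LevelData object, restores collected coins and door states, and moves the player to the saved transform unless its location is zero.
; Checkpoint stores the player transform and saves, while FinishedLevel clears it and saves.
; An existing save that fails the cast is deleted.
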(event Custom|Save%20Game
  (bind _returnvalue (Game|GetCurrentLevelName true))
  (SaveGame|SaveGametoSlot (Variables|Default|GetLevel%20Save) _returnvalue)
  (if true
    (Development|PrintString "Saved Level")
    (else
      (Development|PrintString "No saved level"))))

(event EventBeginPlay
  (Development|PrintString "Loaded into Gm ")
  (bind _returnvalue (Game|GetCurrentLevelName true))
  (bind _returnvalue_2 (SaveGame|DoesSaveGameExist _returnvalue))
  (if _returnvalue_2
    (bind _returnvalue_3 (SaveGame|LoadGamefromSlot _returnvalue))
    (bind _assg_level_data (Utilities|Casting|CastToSG_LevelData _returnvalue_3)
      (:then
        (bind _output_get (Variables|Default|SetLevel%20Save _assg_level_data))
        (Default|LoadCollectedCoins _output_get)
        (Default|LoadDoorStates _output_get)
        (if (not (Class|KismetMathLibrary|EqualExactlyVectorVector (.location (Variables|/Game/Blueprints/NewSaves/SG_LevelData.SG_LevelData_C|GetPlayerTransform (Variables|Default|GetLevel%20Save))) "0, 0, 0"))
          (Transformation|SetWorldTransform (Variables|/Script/Engine.Character|GetCapsuleComponent (Game|GetPlayerCharacter 0)) (Variables|/Game/Blueprints/NewSaves/SG_LevelData.SG_LevelData_C|GetPlayerTransform (Variables|Default|GetLevel%20Save)) false false)))
      (:CastFailed
        (SaveGame|DeleteGameinSlot _returnvalue)))
    (else
      (bind _returnvalue_4 (SaveGame|CreateSaveGameObject "/Game/Blueprints/NewSaves/SG_LevelData.SG_LevelData_C"))
      (Variables|Default|SetLevel%20Save _returnvalue_4))))

(event EventTick
  (params (DeltaSeconds :type Float%20%28single-precision%29)))

(fn ConstructionScript)

(fn Checkpoint
  (params (Player%20Transform :type Transform))
  (Variables|/Game/Blueprints/NewSaves/SG_LevelData.SG_LevelData_C|SetPlayerTransform (Variables|Default|GetLevel%20Save) Player%20Transform)
  (CallFunction|SaveGame))

(fn FinishedLevel
  (Variables|/Game/Blueprints/NewSaves/SG_LevelData.SG_LevelData_C|SetPlayerTransform (Variables|Default|GetLevel%20Save) "")
  (CallFunction|SaveGame))