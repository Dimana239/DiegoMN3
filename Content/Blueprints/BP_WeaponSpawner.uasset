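; BP_WeaponSpawner spawns a random weapon whenever a BP_ThirdPersonCharacter begins overlapping its Sphere1 component.
; SpawnWeapon picks a random row from DT_Weapons and spawns a BP_Weapon at the sphere's transform.
; It writes the row's weapon type, elemental type and base damage into the new weapon's text components.
; Nothing limits repeat spawns, so every qualifying overlap creates another weapon.
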(event OnComponentBeginOverlap(Sphere1)
  (params (OverlappedComponent :type Primitive%20Component%20Object%20Reference) (OtherActor :type Actor%20Object%20Reference) (OtherComp :type Primitive%20Component%20Object%20Reference) (OtherBodyIndex :type Integer) (bFromSweep :type Boolean) (SweepResult :type Hit%20Result%20Structure%20%28by%20ref%29))
  (Utilities|Casting|CastToBP_ThirdPersonCharacter OtherActor)
  (CallFunction|SpawnWeapon))

(event Custom|Spawn%20Weapon
  (bind _outrownames (DataTable|GetDataTableRowNames "/Game/DataTypes/DT_Weapons.DT_Weapons"))
  (bind _returnvalue (Utilities|GetDataTableRow "/Game/DataTypes/DT_Weapons.DT_Weapons" (.OutItem (Utilities|Array|Random _outrownames)))
    (:then
      (bind _returnvalue_2 (Game|SpawnActorfromClass "/Game/Blueprints/BP_Weapon.BP_Weapon_C" (Transformation|GetWorldTransform (Variables|Default|GetSphere1)) "Undefined" "MultiplyWithRoot" 0 0))
      (Rendering|Components|TextRender|SetText (Variables|/Game/Blueprints/BP_Weapon.BP_Weapon_C|GetTextWeaponType _returnvalue_2) (Utilities|Text|ToText(String) (Utilities|String|EnumtoString (.weapontype _returnvalue))))
      (Rendering|Components|TextRender|SetText (Variables|/Game/Blueprints/BP_Weapon.BP_Weapon_C|GetTextElemType _returnvalue_2) (Utilities|Text|ToText(String) (Utilities|String|EnumtoString (.elemetaltype _returnvalue))))
      (Rendering|Components|TextRender|SetText (Variables|/Game/Blueprints/BP_Weapon.BP_Weapon_C|GetTextDmg _returnvalue_2) (Utilities|Text|ToText(Integer) (.basedamage _returnvalue))))))

(event EventBeginPlay)

(event Collision|EventActorBeginOverlap
  (params (OtherActor :type Actor%20Object%20Reference)))

(event EventTick
  (params (DeltaSeconds :type Float%20%28single-precision%29)))

(fn ConstructionScript)