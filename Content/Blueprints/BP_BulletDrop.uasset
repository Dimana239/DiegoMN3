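; Debug actor that visualizes bullet drop by drawing predicted projectile paths.
; BeginPlay takes Start from the Arrow's location, then runs BulletDropCalculator once to draw a line and sphere, overwrite Start with Velocity, lower Velocity's Z and set an unused End.
; It then redraws Predict Projectile Path from those modified values on an endless Delay loop, with collision tracing and timed debug drawing.
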(event Custom|Bullet%20Drop%20Calculator
  (Rendering|Debug|DrawDebugLine :LineStart (Variables|Default|GetStart) :LineEnd (+ (Variables|Default|GetStart) (Variables|Default|GetVelocity)) :Duration (Variables|Default|GetMax%20Sim%20Time))
  (Rendering|Debug|DrawDebugSphere (Variables|Default|GetStart) 1e+02 12 "(R=0.129419,G=0.737008,B=1.000000,A=1.000000)" (Variables|Default|GetMax%20Sim%20Time))
  (Variables|Default|SetStart (Variables|Default|GetVelocity))
  (Variables|Default|SetVelocity (+ (Variables|Default|GetVelocity) "0.000000,0.000000,-1.000000"))
  (Variables|Default|SetEnd (+ (Variables|Default|GetStart) (/ (Variables|Default|GetVelocity) (Math|Vector|MakeVector (Variables|Default|GetSim%20Frequency) 0.0 0.0)))))

(event EventBeginPlay
  (Variables|Default|SetStart (Transformation|GetWorldLocation (Variables|Default|GetArrow)))
  (Utilities|FlowControl|Sequence
    (:then_0
      (CallFunction|BulletDropCalculator))
    (:then_1
      (Class|GameplayStatics|BlueprintPredictProjectilePathAdvanced (Utilities|Struct|MakePredictProjectilePathParams (Variables|Default|GetStart) (Variables|Default|GetVelocity) true 3e+02 (Variables|Default|GetMax%20Sim%20Time) true "ECC_WorldStatic" "ObjectTypeQuery1" 0 (Variables|Default|GetSim%20Frequency) 0.0 "ForDuration" 1.0 false) :!label _label)
      (Utilities|FlowControl|Delay 0.2)
      (goto _label))))

(fn ConstructionScript)