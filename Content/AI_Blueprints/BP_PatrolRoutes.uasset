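; BP_PatrolRoutes is a spline-based patrol route that supplies world-space patrol point locations, presumably for AI.
; Each GetPatrolPointLocation call first advances PatrolIndex by Direction, then returns that spline point's location.
; IncrementPatrolPointsIndex flips Direction to ping-pong along the route, though its upper bound compares the index to spline length rather than point count.
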(event Custom|Increment%20Patrol%20Points%20Index
  (Variables|Default|SetPatrol%20Index (+ (Variables|Default|GetPatrol%20Index) (Variables|Default|GetDirection)))
  (if (>= (Variables|Default|GetPatrol%20Index) (Spline|GetSplineLength (Variables|Default|GetSpline)))
    (Variables|Default|SetDirection -1)
    (elif (<= (Variables|Default|GetPatrol%20Index) 0)
      (Variables|Default|SetDirection 1))))

(fn ConstructionScript)

(fn GetPatrolPointLocation
  (CallFunction|IncrementPatrolPointsIndex)
  (return (Spline|GetLocationatSplinePoint (Variables|Default|GetSpline) (Variables|Default|GetPatrol%20Index) "World")))